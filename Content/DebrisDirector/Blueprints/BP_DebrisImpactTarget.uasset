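; BP_DebrisImpactTarget is an actor that can emit synthetic impact reports through its DebrisReporter for the debris system.
; When EmitImpacts is set, BeginPlay starts a looping timer that calls EmitImpact every EmitInterval.
; Each call reports a simple impact with an upward normal at a fixed height above the actor, randomly jittered horizontally, without any collision or trace.
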(event Custom|EmitImpact
  (Class|DebrisDirectorComponent|ReportImpactSimple (Variables|Default|GetDebrisReporter) (+ (Transformation|GetActorLocation self) (Math|Vector|MakeVector (Math|Random|RandomFloatinRange -45.0 45.0) (Math|Random|RandomFloatinRange -45.0 45.0) 1.5e+02)) (Math|Vector|MakeVector 0.0 0.0 1.0)))

(event EventBeginPlay
  (if (Variables|Default|GetbEmitImpacts)
    (Utilities|Time|SetTimerbyFunctionName self "EmitImpact" (Variables|Default|GetEmitInterval) true)))

(event Collision|EventActorBeginOverlap
  (params (OtherActor :type Actor%20Object%20Reference)))

(event EventTick
  (params (DeltaSeconds :type Float%20%28single-precision%29)))

(fn ConstructionScript)